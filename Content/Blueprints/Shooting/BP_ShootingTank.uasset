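; Multiplayer tank pawn that fires projectiles, tracks health and respawns its player on death.
; Shoot input calls a server event that spawns the projectile at the muzzle.
; Damage lowers clamped Health, whose RepNotify updates the HUD widget created for the locally controlled player.
; At zero health it spawns a death effect, unpossesses, has BP_CustomTankGameMode restart the player, then destroys itself.
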(event `self.ReceiveBeginPlay`
  ; Get Hp
  (set `self.Health` (`self.MaxHealth`))
  (if (`self.IsLocallyControlled`)
    (bind _returnvalue (`|CreateWidget` "/Game/Widgets/WBP_Gameplay.WBP_Gameplay_C"))
    (bind _output_get (set `self.HealthWidgetRef` _returnvalue))
    (`UserWidget.AddToViewport` _output_get 0)
    (`GameplayWidget.OnHealthChanged` _output_get (`self.Health`) (`self.MaxHealth`))))

(event `Server_Shoot`
  ; Shooting(Run oin server)
  (`|SpawnActorFromClass` (`self.ProjectileClass`) (`SceneComponent.K2_GetComponentToWorld` (`self.Muzzle`)) "Undefined" "MultiplyWithRoot" (`GameplayStatics.GetPlayerState` 0) self))

(event `EnhancedInput|/Game/Input/IA_Shoot`
  (params (ActionValue :type Boolean) (ElapsedSeconds :type "Float (double-precision)") (TriggeredSeconds :type "Float (double-precision)") (InputAction :type "InputAction Object Reference" :default "/Game/Input/IA_Shoot.IA_Shoot"))
  ; Shoot
  (:`Started`
    (`self.Server_Shoot`)))

(event `self.ReceiveAnyDamage`
  (params (Damage :type "Float (single-precision)") (DamageType :type "DamageType Object Reference") (InstigatedBy :type "Controller Object Reference") (DamageCauser :type "Actor Object Reference"))
  (bind _returnvalue (`self.GetController`))
  ; Get Damage and send to HP logic
  (`|ExecutionSequence`
    (:`then_0`
      (`self.DamageHealth` Damage))
    (:`then_1`
      (if (<= (`self.Health`) 0.0)
        (`NiagaraFunctionLibrary.SpawnSystemAtLocation` "/Game/Assets/Effects/P_DeathEffect.P_DeathEffect" (`self.K2_GetActorLocation`))
        (bind _asbp_custom_tank_game_mode (cast `/Game/Blueprints/BP_CustomTankGameMode` (`GameplayStatics.GetGameMode`)))
        (set `self.GameModeRef` _asbp_custom_tank_game_mode)
        (set `self.ControllerReference` _returnvalue)
        (`Controller.UnPossess` _returnvalue)
        (`GameModeBase.RestartPlayer` (`self.GameModeRef`) (`self.ControllerReference`))
        (`KismetSystemLibrary.PrintString` (`KismetTextLibrary.Conv_TextToString` (`|FormatText` "Player {playerNum} died!" self)))
        (`self.K2_DestroyActor`)))))

(fn `DamageHealth`
  (params (Damage :type "Float (double-precision)"))
  (set `self.Health` (`KismetMathLibrary.FClamp` (- (`self.Health`) Damage) 0.0 (`self.MaxHealth`))))

(fn `OnRep_Health`
  (bind _healthwidgetref (`self.HealthWidgetRef`))
  (`/Engine/EditorBlueprintResources/StandardMacros.IsValid` _healthwidgetref
    (:`Is Valid`
      (`/Game/Widgets/WBP_Gameplay.UpdateHP_Manual` _healthwidgetref (`self.Health`) (`self.MaxHealth`)))))

(fn `UserConstructionScript`)