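; BP_DamagePowerUp is a powerup that temporarily boosts a shooting tank's projectile damage.
; On activation it casts the tank to BP_ShootingTank, multiplies its ProjectileDamage by DamageMultiplier, and waits for PowerUpDuration.
; It then divides the damage by the same multiplier instead of restoring a saved value, and calls FinishedPowerup.
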(event `self.PowerupActivated`
  (params (SelfTank :type "/Game/Blueprints/BP_Tank Object Reference"))
  (bind _damagemultiplier (`self.DamageMultiplier`))
  (bind _asbp_shooting_tank (cast `/Game/Blueprints/Shooting/BP_ShootingTank` SelfTank))
  (bind _output_get (set `/Game/Blueprints/Shooting/BP_ShootingTank.ProjectileDamage` (* (`/Game/Blueprints/Shooting/BP_ShootingTank.ProjectileDamage` _asbp_shooting_tank) _damagemultiplier) _asbp_shooting_tank))
  (`KismetSystemLibrary.Delay` (`self.PowerUpDuration`))
  (set `/Game/Blueprints/Shooting/BP_ShootingTank.ProjectileDamage` (/ _output_get _damagemultiplier) _asbp_shooting_tank)
  (`self.Finished Powerup`))

(fn `UserConstructionScript`
  (`parent.UserConstructionScript`))