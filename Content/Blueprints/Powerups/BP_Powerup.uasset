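; Base-style powerup pickup actor that a BP_Tank collects by overlapping its box collision.
; The first tank overlap fires PowerupActivated once, which here only prints the tank's name, then destroys the mesh and collision while the actor stays alive.
; A separate FinishedPowerup event destroys the actor; nothing in this graph calls it.
; The PowerUpDuration replication callback is empty.
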(event `PowerupActivated`
  (params (SelfTank :type "/Game/Blueprints/BP_Tank Object Reference"))
  (`KismetSystemLibrary.PrintString` (`KismetTextLibrary.Conv_TextToString` (`|FormatText` "{Tank}: Powerup Activated!" (`KismetSystemLibrary.GetDisplayName` SelfTank)))))

(event `self.BoxCollision.OnComponentBeginOverlap`
  (params (OverlappedComponent :type "PrimitiveComponent Object Reference") (OtherActor :type "Actor Object Reference") (OtherComp :type "PrimitiveComponent Object Reference") (OtherBodyIndex :type Integer) (bFromSweep :type Boolean) (SweepResult :type "HitResult Structure (by ref)"))
  (bind _asbp_tank (cast `/Game/Blueprints/BP_Tank` OtherActor))
  (`/Engine/EditorBlueprintResources/StandardMacros.DoOnce` false
    (:`Completed`
      (`self.PowerupActivated` _asbp_tank)
      (`ActorComponent.K2_DestroyComponent` (`self.PowerUpMesh`))
      (`ActorComponent.K2_DestroyComponent` (`self.BoxCollision`)))))

(event `Finished Powerup`
  (`self.K2_DestroyActor`))

(fn `OnRep_PowerUpDuration`)

(fn `UserConstructionScript`)