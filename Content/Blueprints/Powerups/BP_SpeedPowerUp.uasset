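; BP_SpeedPowerUp is a power-up that temporarily boosts the movement speed of the tank that activates it.
; On activation it multiplies the tank's Speed by SpeedMultiplier, waits PowerUpDuration, then divides by the same multiplier and calls FinishedPowerup.
; The boost is relative, reverting by division instead of restoring a saved original value.
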(event `self.PowerupActivated`
  (params (SelfTank :type "/Game/Blueprints/BP_Tank Object Reference"))
  (bind _speedmultiplier (`self.SpeedMultiplier`))
  (bind _output_get (set `Tank.Speed` (* (`Tank.Speed` SelfTank) _speedmultiplier) SelfTank))
  (`KismetSystemLibrary.Delay` (`self.PowerUpDuration`))
  (set `Tank.Speed` (/ _output_get _speedmultiplier) SelfTank)
  (`self.Finished Powerup`))

(fn `UserConstructionScript`
  (`parent.UserConstructionScript`))